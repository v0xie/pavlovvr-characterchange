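; Trigger volume that switches overlapping BP_CustomCharacterHandler characters to a chosen custom mesh, or restores the default Pavlov character's visibility.
; On overlap, the server gathers handlers inside the trigger, applies the switch, and relays it to clients by RPC.
; A shared switch function sets the mesh and toggles visibility, keeping the Pavlov character visible in debug mode.
; The construction script labels the selected character and hides debug visuals outside debug mode.
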(event OnComponentBeginOverlap(trigger)
  (params (OverlappedComponent :type Primitive%20Component%20Object%20Reference) (OtherActor :type Actor%20Object%20Reference) (OtherComp :type Primitive%20Component%20Object%20Reference) (OtherBodyIndex :type Integer) (bFromSweep :type Boolean) (SweepResult :type Hit%20Result%20Structure%20%28by%20ref%29))
  ;[1 1 1] Tick
  (Networking|SwitchHasAuthority
    (:Authority
      ;[1 1 1] Set custom mesh
      (bind _overlappingcustomcharacters_ (CallFunction|GetOverlappingCustomCharacters))
      (if _overlappingcustomcharacters_
        (for _array_element (Variables|Default|GetOverlappingCustomCharacters)
          (CallFunction|RPCAdd _array_element (Variables|Default|GetCustomCharacterToSwitchTo)))
        (Utilities|FlowControl|Delay 0.25)
        (Utilities|Array|Clear (Variables|Default|GetOverlappingCustomCharacters))))))

(event Custom|RPC_Add_TellClients
  (params (BPCustomChar :type BP%20Custom%20Character%20Handler%20Object%20Reference) (CustomCharacterToSwitchTo :type Enum_CustomCharacters%20Enum :default "NewEnumerator0"))
  ;[1 1 1] Model switching logic
  (Networking|SwitchHasAuthority
    (:Remote
      (CallFunction|HandleCharacterSwitch BPCustomChar CustomCharacterToSwitchTo))))

(event Custom|RPC_Add
  (params (BPCustomChar :type BP%20Custom%20Character%20Handler%20Object%20Reference) (CustomCharacterToSwitchTo :type Enum_CustomCharacters%20Enum :default "NewEnumerator0"))
  ;[1 1 1] Model switching logic
  (Networking|SwitchHasAuthority
    (:Authority
      (Utilities|FlowControl|Sequence
        (:then_0
          (CallFunction|HandleCharacterSwitch BPCustomChar CustomCharacterToSwitchTo))
        (:then_1
          (CallFunction|RPCAddTellClients BPCustomChar CustomCharacterToSwitchTo))))))

(fn ConstructionScript
  (Utilities|FlowControl|Sequence
    (:then_0
      (if (Variables|Default|GetbRestorePavSkelVisibility)
        ;[1 1 1] Comment
        (Rendering|Components|TextRender|SetText (Variables|Default|Getcharacter_name) (Utilities|Text|MakeLiteralText "Default"))
        (else
          (switch Utilities|FlowControl|Switch|SwitchonEnum_CustomCharacters (Variables|Default|GetCustomCharacterToSwitchTo)
            (:NewEnumerator0
              ;[1 1 1] Comment
              (Rendering|Components|TextRender|SetText (Variables|Default|Getcharacter_name) (Utilities|Text|MakeLiteralText "Red Mannequin")))
            (:NewEnumerator1
              (Rendering|Components|TextRender|SetText (Variables|Default|Getcharacter_name) (Utilities|Text|MakeLiteralText "Green Mannequin")))
            (:NewEnumerator2
              (Rendering|Components|TextRender|SetText (Variables|Default|Getcharacter_name) (Utilities|Text|MakeLiteralText "Blue Mannequin")))))))
    (:then_1
      (if (not (Variables|Default|GetbDebugMode))
        (Rendering|SetVisibility (Variables|Default|Getdebug) false false)))))

(fn GetOverlappingCustomCharacters
  (bind _trigger (Variables|Default|Gettrigger))
  (bind _overlappingactors (Collision|GetOverlappingActors _trigger "/Game/CustomCharacter/Blueprints/BP_CustomCharacterHandler.BP_CustomCharacterHandler_C" :!class /Script/Engine.PrimitiveComponent))
  (if (> (Utilities|Array|Length _overlappingactors) 0)
    (for _array_element _overlappingactors
      (bind _asbp_custom_character_handler (Utilities|Casting|CastToBP_CustomCharacterHandler _array_element))
      (Utilities|Array|AddUnique (Variables|Default|GetOverlappingCustomCharacters) _asbp_custom_character_handler))
    (return true)
    (else
      (return false))))

(fn HandleCharacterSwitch
  (params (CustomCharacter :type BP%20Custom%20Character%20Handler%20Object%20Reference) (Enum :type Enum_CustomCharacters%20Enum :default "NewEnumerator0"))
  (Default|SetCustomCharacterMesh CustomCharacter Enum)
  (if (Variables|Default|GetbRestorePavSkelVisibility)
    (Default|SetPavlovCharacterVisibility CustomCharacter true)
    (Default|SetCustomCharacterVisibility CustomCharacter false)
    (else
      (Default|SetCustomCharacterVisibility CustomCharacter true)
      (Default|SetPavlovCharacterVisibility CustomCharacter (Variables|Default|GetbDebugMode)))))