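; Custom character actor that attaches to a Pavlov player's pawn and overlays a selectable skeletal mesh, hidden from the owner.
; The mesh follows the Pavlov skeleton through master pose or a copy-pose AnimBP that falls back to master pose, with height-based scaling on authority.
; Visibility functions swap custom and Pavlov meshes, keeping hidden Pavlov bones ticking.
; When killable, the server removes it after a delay upon a "dead" tag or invalid PlayerState.
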(event EventTick
  (params (DeltaSeconds :type Float%20%28single-precision%29))
  ;[1 1 1] Handle killing self on player tag 'dead'
  (Utilities|FlowControl|Sequence
    (:then_0
      (if (and (Variables|Default|GetEnableKillable) (Variables|Default|GetbIsPlayerControlled))
        (Utilities|FlowControl|Sequence
          (:then_0
            (Networking|SwitchHasAuthority
              (:Authority
                (if (Math|Boolean|ORBoolean (not (Utilities|IsValid (Variables|Default|GetOwningPlayerState))) (Actor|ActorHasTag (Components|GetOwner) "dead") (Actor|ActorHasTag self "dead") (Actor|ActorHasTag (Variables|Default|GetOwningPlayerState) "dead"))
                  ;[1 1 1] Kill self
                  (Utilities|FlowControl|DoOnce false
                    (:Completed
                      (Utilities|FlowControl|Delay (Variables|Default|GetfRagdollLifespanAfterDeath))
                      (CallFunction|KillCharacterDead)))))))
          (:then_1
            (if (Variables|Default|GetbUseMasterPoseComponent)
              (Networking|SwitchHasAuthority
                (:Authority
                  _)
                (:Remote
                  _))
              ;[1 1 1] Set mesh to copy using Master Pose Component
              (if (Utilities|IsValid (Variables|Default|GetPavlovSkelMeshToCopy))
                (Utilities|FlowControl|DoOnce false :!label _label
                  (:Completed
                    (Class|SkinnedMeshComponent|SetMasterPoseComponent (Variables|Character|GetMesh) (Variables|Default|GetPavlovSkelMeshToCopy) true)
                    (CallFunction|ScaleCustomSkeltoMatchPavlovSkel) ; might not be necessary? probly is
                  )))
              (else
                ;[1 1 1] Use copy pose as mesh
                (Networking|SwitchHasAuthority
                  (:Authority
                    _)
                  (:Remote
                    _))
                (if (Utilities|IsValid (Variables|Default|GetPavlovSkelMeshToCopy))
                  (Utilities|FlowControl|DoOnce false
                    (:Completed
                      (bind _success (CallFunction|SetupCopyPoseasMesh))
                      (if _success ; falls back to master pose component
                        (Components|Animation|SetAnimationMode (Variables|Character|GetMesh) "AnimationBlueprint")
                        (CallFunction|ScaleCustomSkeltoMatchPavlovSkel)
                        (else
                          (goto _label))))))))))))))

(event EventBeginPlay
  (bind _returnvalue (Transformation|GetActorLocation))
  (bind _mesh (Variables|Character|GetMesh))
  (bind (_x _y) (Math|Vector|BreakVector _returnvalue))
  (bind _returnvalue_2 (Transformation|GetWorldLocation _mesh))
  (bind (_x_2 _y_2) (Math|Vector|BreakVector _returnvalue_2))
  ;[1 1 1] BeginPlay
  (Utilities|FlowControl|Sequence
    (:then_0
      ;[1 1 1] Comment
      (Networking|SwitchHasAuthority ; This must run on client and server for client to see\nplayer mesh being copied
        (:Authority
          _)
        (:Remote
          _))
      (if (Utilities|IsValid (Variables|Default|GetOwningPlayerState))
        (bind (_pavlovskeletalmesh _pavlovsatchelmesh) (CallFunction|GetPavlovSkeleton (Variables|Default|GetOwningPlayerState)))
        (Variables|Default|SetPavlovSkelMeshToCopy _pavlovskeletalmesh)
        (Variables|Default|SetSatchelMesh _pavlovsatchelmesh)
        ;[1 1 1] Set capsule height
        (bind _playerstatus (Class|PavlovProxyStatics|GetPavlovPlayerStatus (Variables|Default|GetOwningPlayerState)))
        (if (CallFunction|IsPavPawn? (.Pawn (Utilities|Struct|BreakPavlovPlayerStatus _playerstatus)))
          ;[1 1 1] Attach and set transforms on new model
          (Transformation|AttachActorToActor (.Pawn (Utilities|Struct|BreakPavlovPlayerStatus _playerstatus)) "root" "SnapToTarget" "SnapToTarget" "SnapToTarget" true)
          (Transformation|AttachComponentToComponent (Variables|Character|GetMesh) (Variables|Default|GetPavlovSkelMeshToCopy) "None" "KeepRelative" "SnapToTarget" "SnapToTarget" true)
          (Transformation|SetActorLocation (Math|Vector|MakeVector _x _y (.Z (Math|Vector|BreakVector (Transformation|GetSocketLocation (Variables|Default|GetPavlovSkelMeshToCopy) "root")))) false true)
          (Transformation|SetWorldLocation _mesh (Math|Vector|MakeVector _x_2 _y_2 0.0) false false)
          (Class|PrimitiveComponent|SetOwnerNoSee (Variables|Character|GetMesh) true) ; Hides custom model from pawn owner\nIf disabled, player can see their body
        )))
    (:then_1
      (Variables|Default|SetEnableKillable true))))

(event EventRoundStarted)

(event EventRoundStandby)

(event EventRoundEnded)

(event EventRoundStarting)

(fn ConstructionScript
  (Utilities|FlowControl|Sequence
    (:then_0
      (if (Variables|Default|GetbPavlovMeshVisibilityOnSpawn)
        (CallFunction|SetCustomCharacterVisibility false)
        (CallFunction|SetPavlovCharacterVisibility true)
        (else
          (CallFunction|SetCustomCharacterVisibility true)
          (CallFunction|SetPavlovCharacterVisibility false))))
    (:then_1
      (CallFunction|SetCustomCharacterMesh (Variables|Default|GetCustomCharacterMesh)))))

(fn SetPavlovCharacterVisibility
  (params (PavlovMeshVisible :type Boolean))
  (bind _pavlovskelmeshtocopy (Variables|Default|GetPavlovSkelMeshToCopy))
  (bind _satchelmesh (Variables|Default|GetSatchelMesh))
  (if (and (Utilities|IsValid (Variables|Default|GetPavlovSkelMeshToCopy)) (Utilities|IsValid (Variables|Default|GetSatchelMesh)))
    (if PavlovMeshVisible
      ;[1 1 1] Turn on visibility of pavlov mesh
      (Rendering|SetVisibility (Variables|Default|GetPavlovSkelMeshToCopy) true false)
      (Rendering|SetVisibility (Variables|Default|GetSatchelMesh) true false)
      (Variables|/Script/Engine.SkinnedMeshComponent|SetbEnableUpdateRateOptimizations (Variables|Default|GetPavlovSkelMeshToCopy) true)
      (Variables|/Script/Engine.SkinnedMeshComponent|SetbEnableUpdateRateOptimizations (Variables|Default|GetSatchelMesh) true)
      (else
        ;[1 1 1] Turn off visibility of pavlov mesh
        (Rendering|SetVisibility (Variables|Default|GetPavlovSkelMeshToCopy) false false)
        (Rendering|SetVisibility (Variables|Default|GetSatchelMesh) false false)
        (Variables|/Script/Engine.SkinnedMeshComponent|SetbEnableUpdateRateOptimizations _pavlovskelmeshtocopy false)
        (Variables|/Script/Engine.SkinnedMeshComponent|SetVisibilityBasedAnimTickOption _pavlovskelmeshtocopy "AlwaysTickPoseAndRefreshBones")
        (Variables|/Script/Engine.SkinnedMeshComponent|SetbEnableUpdateRateOptimizations _satchelmesh false)
        (Variables|/Script/Engine.SkinnedMeshComponent|SetVisibilityBasedAnimTickOption _satchelmesh "AlwaysTickPoseAndRefreshBones")))))

(fn SetCustomCharacterVisibility
  (params (CustomCharacterVisibility :type Boolean))
  (if CustomCharacterVisibility
    ;[1 1 1] Turn on visibility of custom mesh
    (Rendering|SetVisibility (Variables|Character|GetMesh) true true)
    (Variables|Default|SetbCustomCharacterIsVisible true)
    (else
      ;[1 1 1] Turn off visibility of custom mesh
      (Rendering|SetVisibility (Variables|Character|GetMesh) false true)
      (Variables|Default|SetbCustomCharacterIsVisible false))))

(fn ToggleCustomCharacterVisibility
  (if (Variables|Default|GetbCustomCharacterIsVisible)
    (CallFunction|SetCustomCharacterVisibility false)
    (CallFunction|SetPavlovCharacterVisibility true)
    (else
      (CallFunction|SetPavlovCharacterVisibility false)
      (CallFunction|SetCustomCharacterVisibility true))))

(fn ScaleCustomSkeltoMatchPavlovSkel
  (Networking|SwitchHasAuthority
    (:Authority
      (bind _distancefromheadtoroot (CallFunction|GetHeightOfSkeletalMesh (Variables|Character|GetMesh))) ; CustomCharacter
      (bind _distancefromheadtoroot_2 (CallFunction|GetHeightOfSkeletalMesh (Variables|Default|GetPavlovSkelMeshToCopy))) ; PavlovSkeleton
      (Transformation|SetWorldScale3D (Variables|Transformation|GetRootComponent) (Math|Vector|MakeVector (* (/ _distancefromheadtoroot_2 _distancefromheadtoroot) (Variables|Default|GetGlobalCharacterScaleScalar)) (* (/ _distancefromheadtoroot_2 _distancefromheadtoroot) (Variables|Default|GetGlobalCharacterScaleScalar)) (* (/ _distancefromheadtoroot_2 _distancefromheadtoroot) (Variables|Default|GetGlobalCharacterScaleScalar)))))))

(fn SetCustomCharacterMesh
  (params (CustomCharacterMesh :type Enum_CustomCharacters%20Enum :default "NewEnumerator0"))
  (bind _mesh (Variables|Character|GetMesh))
  (bind _mesh_2 (Variables|Character|GetMesh))
  (bind _mesh_3 (Variables|Character|GetMesh))
  ;[1 1 1] Per character setup: Set model here
  (Utilities|FlowControl|Sequence
    (:then_0
      (Utilities|FlowControl|DoOnce false
        (:Completed
          (switch Utilities|FlowControl|Switch|SwitchonEnum_CustomCharacters CustomCharacterMesh :!label _label
            (:NewEnumerator0
              (Class|SkinnedMeshComponent|SetSkeletalMesh _mesh_2 "/Game/CustomCharacter/Characters/UE4_Mannequin/Mesh/SK_Mannequin.SK_Mannequin" false)
              (Rendering|Material|SetMaterial _mesh_2 0 "/Game/CustomCharacter/Characters/UE4_Mannequin/Materials/MI_UE4Man_Body_0.MI_UE4Man_Body_0")
              (Variables|Default|SetGlobalCharacterScaleScalar 1.1))
            (:NewEnumerator1
              (Class|SkinnedMeshComponent|SetSkeletalMesh _mesh_3 "/Game/CustomCharacter/Characters/UE4_Mannequin/Mesh/SK_Mannequin.SK_Mannequin" false)
              (Rendering|Material|SetMaterial _mesh_3 0 "/Game/CustomCharacter/Characters/UE4_Mannequin/Materials/MI_UE4Man_Body_1.MI_UE4Man_Body_1")
              (Variables|Default|SetGlobalCharacterScaleScalar 1.1))
            (:NewEnumerator2
              (Class|SkinnedMeshComponent|SetSkeletalMesh _mesh "/Game/CustomCharacter/Characters/UE4_Mannequin/Mesh/SK_Mannequin.SK_Mannequin" false)
              (Rendering|Material|SetMaterial _mesh 0 "/Game/CustomCharacter/Characters/UE4_Mannequin/Materials/MI_UE4Man_Body_2.MI_UE4Man_Body_2")
              (Variables|Default|SetGlobalCharacterScaleScalar 1.1)))
          (Variables|Default|SetCustomCharacterMesh CustomCharacterMesh))))
    (:then_1
      (if (Utilities|Enum|NotEqual(Enum) CustomCharacterMesh (Variables|Default|GetCustomCharacterMesh))
        (goto _label)))))

(fn KillCharacterDead
  (CallFunction|SetPavlovCharacterVisibility false)
  (CallFunction|SetCustomCharacterVisibility false)
  (Actor|SetLifeSpan 1.0))

(fn SetupCopyPoseasMesh
  (bind _mesh (Variables|Character|GetMesh))
  (bind _mesh_2 (Variables|Character|GetMesh))
  (bind _returnvalue (Components|SkeletalMesh|GetAnimInstance _mesh_2))
  (switch Utilities|FlowControl|Switch|SwitchonEnum_CustomCharacters (Variables|Default|GetCustomCharacterMesh)
    (:NewEnumerator0
      ;[1 1 1] Character 0 Setup
      (Components|SkeletalMesh|SetAnimInstanceClass _mesh "/Game/CustomCharacter/Characters/UE4_Mannequin/Mesh/BP_Mannequin_AnimBlueprint.BP_Mannequin_AnimBlueprint_C") ; Set the anim blueprint of the character
      (bind _asbp_mannequin_anim_blueprint (Utilities|Casting|CastToBP_Mannequin_AnimBlueprint _returnvalue) ; Set cast to the anim blueprint you want
        (:then
          _)
        (:CastFailed
          (return false))))
    (:NewEnumerator1
      ;[1 1 1] Character 1 Setup
      (Components|SkeletalMesh|SetAnimInstanceClass _mesh "/Game/CustomCharacter/Characters/UE4_Mannequin/Mesh/BP_Mannequin_AnimBlueprint.BP_Mannequin_AnimBlueprint_C")
      (bind _asbp_mannequin_anim_blueprint_2 (Utilities|Casting|CastToBP_Mannequin_AnimBlueprint _returnvalue)
        (:then
          _)
        (:CastFailed
          (return false))))
    (:NewEnumerator2
      ;[1 1 1] Character 2 Setup
      (Components|SkeletalMesh|SetAnimInstanceClass _mesh "/Game/CustomCharacter/Characters/UE4_Mannequin/Mesh/BP_Mannequin_AnimBlueprint.BP_Mannequin_AnimBlueprint_C")
      (bind _asbp_mannequin_anim_blueprint_3 (Utilities|Casting|CastToBP_Mannequin_AnimBlueprint _returnvalue)
        (:then
          _)
        (:CastFailed
          (return false)))))
  (Default|SetMeshtoCopy _asbp_mannequin_anim_blueprint_3 (Variables|Default|GetPavlovSkelMeshToCopy))
  (return true))