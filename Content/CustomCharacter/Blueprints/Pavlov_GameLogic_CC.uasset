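; Pavlov VR game mode logic template that gives each spawning player a replicated BP_CustomCharacterHandler as a custom character.
; The server runs round states with delays and a match timer, grants cash and buy time, and tags dead players.
; It tracks players on spawn, working around broken OnPlayerJoined, and relays round changes to BPI_MatchRounds actors.
; Helper functions and unwired example nodes demonstrate the API; team assignment is a placeholder.
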(event Custom|End%20Match
  ;[1 1 1 1 170] Round-Based Logic
  ;;[1 1 1] Time till match ends
  ;; End match can be called due to specific requirements being met vs having it on a timer.
  (Utilities|FlowControl|DoOnce false
    (:Completed
      (bind _asgame_mode (Utilities|Casting|CastToGameMode (Game|GetGameMode)))
      (Class|GameMode|EndMatch _asgame_mode))))

(event Custom|Play%20Sound%20FX%202D
  (params (Sound :type Sound%20Base%20Object%20Reference))
  ;[1 1 1] Example of replicated 2d sound effect (make sure to call from server)
  (Audio|PlaySound2D Sound 1.0 1.0 0.0 0 0))

(event Custom|Match%20Timer
  ;[1 1 1 1 170] Round-Based Logic
  ;;[1 1 1] Time till match ends
  ;; End match can be called due to specific requirements being met vs having it on a timer.
  (Utilities|Time|SetTimerbyEvent (delegate Custom|End%20Match) 6e+02))

(event Custom|Play%20Sound%20FX%20At%20Location
  (params (Sound :type Sound%20Base%20Object%20Reference) (Location :type Vector))
  ;[1 1 1] Example of replicated sound that plays at a location (use cues for attenuation, call from server)
  (Audio|PlaySoundatLocation Sound Location "0, 0, 0" 1.0 1.0 0.0 0 0 0))

(event Custom|CustomOnPlayerJoined
  (params (PlayerStatus :type Pavlov%20Player%20Status%20Structure))
  (bind (_playerstate _controller _pawn) (Utilities|Struct|BreakPavlovPlayerStatus PlayerStatus))
  (bind _array (Utilities|Array|MakeArray "None"))
  ;[1 0.3263 0.3123 1 170] Custom Character Logic
  ;;[1 1 1] Custom OnPlayerJoined (called on spawn). Normal OnPlayerJoined is broken
  (Utilities|Array|AddUnique (Variables|Default|GetConnectedPlayers) _playerstate)
  (Variables|/Script/Engine.Actor|SetTags _controller _array)
  (Variables|/Script/Engine.Actor|SetTags _pawn _array))

(event Custom|SpawnCustomCharacter
  (params (PlayerStatus :type Pavlov%20Player%20Status%20Structure) (CharacterRagdollTime :type Float%20%28single-precision%29))
  (bind (_playerstate _controller _pawn) (Utilities|Struct|BreakPavlovPlayerStatus PlayerStatus))
  ;[1 0.3263 0.3123 1 170] Custom Character Logic
  ;;[1 1 1] Spawn CustomCharacter
  (Networking|SwitchHasAuthority
    (:Authority
      (bind _returnvalue (Game|SpawnActorfromClass "/Game/CustomCharacter/Blueprints/BP_CustomCharacterHandler.BP_CustomCharacterHandler_C" (Transformation|GetActorTransform _pawn) "AlwaysSpawn" _pawn _playerstate (Variables|Default|GetGlobalRagdollLifespan) true "NewEnumerator0" true true 0))
      (Networking|SetReplicates _returnvalue true)
      (Class|ActorComponent|SetIsReplicated (Variables|/Script/Engine.Character|GetMesh _returnvalue) true))))

(event EventOnRoundEnd
  ;[1 1 1 1 170] Round-Based Logic
  ;;[1 1 1] On Round End, change delays duration to adjust the wait for players to respawn and prepare before the match starts
  (Development|PrintString "Round End Declare Winner")
  (CallFunction|PlaySoundFX2D)
  (bind _players (CallFunction|GetPlayers))
  (for _array_element _players
    (bind (_playerstatus _bsucceeded) (Class|PavlovProxyStatics|GetPavlovPlayerStatus _array_element))
    (if _bsucceeded
      (if (not (.bDead (Utilities|Struct|BreakPavlovPlayerStatus _playerstatus)))
        (CallFunction|ManageTags (.PlayerState (Utilities|Struct|BreakPavlovPlayerStatus _playerstatus)) true "dead")
        (Game|Damage|ApplyDamage 0 9999.0 0 0))))
  (Utilities|FlowControl|Delay 3.0)
  (Class|PavlovGameLogic|SetRoundState "Starting")
  (Class|PavlovGameLogic|SetMovementDisabled true)
  (for _array_element_2 (Variables|Default|GetConnectedPlayers)
    (Class|PavlovGameLogic|SetPlayerBuyingEnabled _array_element_2 15.0 1e+03))
  (Utilities|FlowControl|Delay 2.0)
  (Class|PavlovGameLogic|SetRoundState "StandBy")
  (Utilities|FlowControl|Delay 5.0)
  (Class|PavlovGameLogic|SetRoundState "Started")
  (Class|PavlovGameLogic|SetMovementDisabled false)
  (CallFunction|PlaySoundFX2D))

(event EventBeginPlay
  ;[1 1 1 1 170] Round-Based Logic
  ;;[1 1 1] Time till game starts
  (Networking|SwitchHasAuthority
    (:Authority
      (Utilities|FlowControl|Delay 2.0)
      (Class|PavlovGameLogic|SetRoundState "StandBy")
      (Utilities|FlowControl|Delay 3.0)
      (Class|PavlovGameLogic|SetRoundState "Started")
      (CallFunction|MatchTimer))))

(event EventOnPlayerKilled
  (params (PlayerStatus :type Pavlov%20Player%20Status%20Structure%20%28by%20ref%29) (Killer :type Player%20State%20Object%20Reference))
  (bind (_playerstate _controller _pawn) (Utilities|Struct|BreakPavlovPlayerStatus PlayerStatus))
  (bind _array (Utilities|Array|MakeArray "dead"))
  ;[1 0.3263 0.3123 1 170] Custom Character Logic
  ;;[1 1 1] On Player Killed
  (Networking|SwitchHasAuthority
    (:Authority
      (CallFunction|ManageTags _playerstate true "dead")
      (Variables|/Script/Engine.Actor|SetTags _controller _array)
      (Variables|/Script/Engine.Actor|SetTags _pawn _array))))

(event EventOnRoundStateChanged
  (params (OldState :type EPavlovRoundState%20Enum :default "Starting") (NewState :type EPavlovRoundState%20Enum :default "Starting"))
  ;[1 1 1 1 170] Round-Based Logic
  ;;[1 1 1] Updates all blueprints with BPI_MatchRounds implemented,
  ;;  can be used to reset actors to initial state (Ill cover this in the video)
  (CallFunction|RoundInterfaceCall NewState)
  (Development|PrintString (Utilities|String|Append (Utilities|String|EnumtoString OldState) "||" (Utilities|String|EnumtoString NewState))))

(event EventOnRoundBegin
  ;[1 1 1 1 170] Round-Based Logic
  ;;[1 1 1] OnRoundBegin
  (Class|PavlovGameLogic|PostRoundCleanUp)
  (Utilities|FlowControl|Delay 1.0)
  (Class|PavlovGameLogic|SpawnandPosessPawns)
  (Development|PrintString "Round Start"))

(event EventOnCustomGameModeInit
  ;[1 1 1] Init GameMode Properties when server starts
  (Class|PavlovGameLogic|SetGameModeProperties (Utilities|Struct|MakePavlovGameModeProperties false true false 99999 10000 0 false true 5.0 false false 30 10 true false 45)))

(event EventOnPlayerLeftServer
  (params (PlayerStatus :type Pavlov%20Player%20Status%20Structure%20%28by%20ref%29))
  (bind (_playerstate _controller _pawn) (Utilities|Struct|BreakPavlovPlayerStatus PlayerStatus))
  (bind _array (Utilities|Array|MakeArray "dead"))
  ;[1 0.3263 0.3123 1 170] Custom Character Logic
  ;;[1 1 1] OnPlayerLeftServer
  (Utilities|Array|RemoveItem (Variables|Default|GetConnectedPlayers) _playerstate)
  (CallFunction|ManageTags _playerstate true "dead")
  (Variables|/Script/Engine.Actor|SetTags _controller _array)
  (Variables|/Script/Engine.Actor|SetTags _pawn _array))

(event EventOnPlayerSpawned
  (params (PlayerStatus :type Pavlov%20Player%20Status%20Structure%20%28by%20ref%29))
  (bind (_playerstate _controller _pawn) (Utilities|Struct|BreakPavlovPlayerStatus PlayerStatus))
  (bind _array (Utilities|Array|MakeArray "None"))
  ;[1 0.3263 0.3123 1 170] Custom Character Logic
  ;;[1 1 1] On Player Spawn (Thanks Dean for the spawn logic)
  (Networking|SwitchHasAuthority
    (:Authority
      (if (== (Utilities|Array|FindItem (Variables|Default|GetConnectedPlayers) _playerstate) -1)
        (CallFunction|CustomonPlayerJoined PlayerStatus) ; Custom
      )
      (CallFunction|ManageTags _playerstate false "dead")
      (Variables|/Script/Engine.Actor|SetTags _controller _array)
      (Variables|/Script/Engine.Actor|SetTags _pawn _array)
      (Class|PavlovGameLogic|SetPlayerBuyingEnabled _playerstate 1.2e+02 1e+03)
      (Class|PavlovGameLogic|GivePlayerCash _playerstate 8100)
      (CallFunction|SpawnCustomCharacter PlayerStatus 4.9))))

(fn ConstructionScript)

(fn GetConnectedPawns
  (for _array_element (Variables|Default|GetConnectedPlayers)
    (bind (_playerstatus _bsucceeded) (Class|PavlovProxyStatics|GetPavlovPlayerStatus _array_element))
    (if _bsucceeded
      (if (CallFunction|IsPavPawn? (.Pawn (Utilities|Struct|BreakPavlovPlayerStatus _playerstatus)))
        (Math|Integer|IncrementInt (LocalVariables|GetL_AliveCount)
          (:%20%20
            (Utilities|Array|AddUnique (LocalVariables|GetL_AlivePawns) (.Pawn (Utilities|Struct|BreakPavlovPlayerStatus _playerstatus)))))
        (else
          (Math|Integer|IncrementInt (LocalVariables|GetL_GhostCount)
            (:%20%20
              (Utilities|Array|AddUnique (LocalVariables|GetL_GhostPawns) (.Pawn (Utilities|Struct|BreakPavlovPlayerStatus _playerstatus)))))))))
  (return (LocalVariables|GetL_AlivePawns) (LocalVariables|GetL_AliveCount) (LocalVariables|GetL_GhostPawns) (LocalVariables|GetL_GhostCount)))

(fn RoundInterfaceCall
  (params (Round%20State :type EPavlovRoundState%20Enum :default "Starting"))
  (bind _outactors (Actor|GetAllActorswithInterface "/CustomMapTools/Blueprints/BPI_MatchRounds.BPI_MatchRounds_C"))
  (LocalVariables|SetL_InterfaceActors _outactors)
  (switch Utilities|FlowControl|Switch|SwitchonEPavlovRoundState Round%20State
    (:Starting
      (Class|BPIMatchRounds|RoundStarting(Message) (LocalVariables|GetL_InterfaceActors)))
    (:StandBy
      (Class|BPIMatchRounds|RoundStandby(Message) (LocalVariables|GetL_InterfaceActors)))
    (:Started
      (Class|BPIMatchRounds|RoundStarted(Message) (LocalVariables|GetL_InterfaceActors)))
    (:Ended
      (Class|BPIMatchRounds|RoundEnded(Message) (LocalVariables|GetL_InterfaceActors))))
  (return))

(fn RespawnPlayer
  (params (PlayerStatus :type Pavlov%20Player%20Status%20Structure%20%28by%20ref%29) (As%20Ghost :type Boolean) (Spawn%20At%20Transform? :type Boolean) (Transform :type Transform))
  (bind _controller (Utilities|Struct|BreakPavlovPlayerStatus PlayerStatus))
  (if Spawn%20At%20Transform?
    (Class|PavlovGameLogic|Spawn _controller Transform As%20Ghost)
    (else
      (bind _transform (Class|PavlovGameLogic|GetSpawnTransform _controller))
      (Class|PavlovGameLogic|Spawn _controller _transform As%20Ghost)))
  (return))

(fn OnAssignTeam
  (params (Status :type Pavlov%20Player%20Status%20Structure%20%28by%20ref%29))
  (bind _returnvalue (Class|KismetSystemLibrary|MakeLiteralInteger))
  (if (> _returnvalue _returnvalue)
    (return 0)
    (else
      (return 1))))

(fn GetPavSkel
  (params (PavPawn :type Pawn%20Object%20Reference))
  (if (CallFunction|IsPavPawn? PavPawn)
    (bind _ascharacter (Utilities|Casting|CastToCharacter PavPawn)
      (:then
        (return (Utilities|Array|Get(acopy) (Actor|GetComponentsByClass _ascharacter "/Script/Engine.SkeletalMeshComponent") 1) true))
      (:CastFailed
        (return 0 false)))))

(fn GetHeightOfSkel
  (params (Mesh :type Skeletal%20Mesh%20Component%20Object%20Reference))
  (return (Class|KismetAnimationLibrary|DistanceBetweenTwoSocketsandMapRange Mesh "root" "RTS_World" "head" "RTS_World" false 0.0 0.0 0.0 0.0)))

(fn GetOwnedCustomCharacter
  (params (Pawn :type Pawn%20Object%20Reference))
  (for _array_element (Actor|GetAllChildActors Pawn true)
    (bind _asbp_custom_character_handler (Utilities|Casting|CastToBP_CustomCharacterHandler _array_element))
    (return _asbp_custom_character_handler true))
  (return 0 false))

(fn GetPlayers
  (bind _asgame_state (Utilities|Casting|CastToGameState (Game|GetGameState)))
  (return (Variables|/Script/Engine.GameStateBase|GetPlayerArray _asgame_state)))