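; Blueprint function library for the custom character system that looks up Pavlov player meshes and measures skeletal mesh height.
; GetPavlovSkeleton resolves a PlayerState to a validated Pavlov pawn, returning its Character, body mesh and satchel mesh.
; The meshes are picked by hard-coded component array indices, so results depend on the pawn's component order.
; GetHeightOfSkeletalMesh measures world-space distance between the root and head bones.
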(fn GetPavlovSkeleton
  (params (PlayerState :type Player%20State%20Object%20Reference))
  (bind (_playerstatus _bsucceeded) (Class|PavlovProxyStatics|GetPavlovPlayerStatus PlayerState))
  (if (and _bsucceeded (CallFunction|IsPavPawn? (.Pawn (Utilities|Struct|BreakPavlovPlayerStatus _playerstatus))))
    (bind _ascharacter (Utilities|Casting|CastToCharacter (.Pawn (Utilities|Struct|BreakPavlovPlayerStatus _playerstatus)))
      (:then
        (return (Utilities|Array|Get(acopy) (Actor|GetComponentsByClass _ascharacter "/Script/Engine.SkeletalMeshComponent") 1) (Utilities|Array|Get(acopy) (Actor|GetComponentsByClass (.Pawn (Utilities|Struct|BreakPavlovPlayerStatus _playerstatus)) "/Script/Engine.SkinnedMeshComponent") 4) _ascharacter))
      (:CastFailed
        _)))
  (return 0 0 0))

(fn GetHeightOfSkeletalMesh
  (params (SkelMesh :type Skeletal%20Mesh%20Component%20Object%20Reference))
  (return (Class|KismetAnimationLibrary|DistanceBetweenTwoSocketsandMapRange SkelMesh "root" "RTS_World" "head" "RTS_World" false 0.0 0.0 0.0 0.0)))